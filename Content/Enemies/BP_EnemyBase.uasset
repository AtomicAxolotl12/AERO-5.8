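; Base enemy Blueprint that roams the navmesh at random and chases pawns it sees.
; Roaming loops AI MoveTo to random nearby points after each successful move.
; PawnSensing redirects movement to the seen pawn, with a retriggerable delay resuming roaming once sightings stop.
; Tick sets a random rotation every frame, and the DamageArea overlap checks the "Character" tag but applies no damage.
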(event `self.ReceiveBeginPlay`
  (`self.Random Roaming`))

(event `Random Roaming`
  (bind _randomlocation (`NavigationSystemV1.K2_GetRandomLocationInNavigableRadius` (`self.K2_GetActorLocation`) 1500.0 null null))
  (`|AIMoveTo` self _randomlocation null
    (:`OnSuccess`
      (`KismetSystemLibrary.Delay` 0.2)
      (`self.Random Roaming`))))

(event `self.PawnSensing.OnSeePawn`
  (params (Pawn :type "Pawn Object Reference"))
  (`|ExecutionSequence`
    (:`then_0`
      (`|AIMoveTo` self (0.0 0.0 0.0) Pawn))
    (:`then_1`
      (`KismetSystemLibrary.RetriggerableDelay` 1.0)
      (`self.Random Roaming`))))

(event `self.ReceiveTick`
  (params (DeltaSeconds :type "Float (single-precision)"))
  (`self.K2_SetActorRotation` (`KismetMathLibrary.RandomRotator` true)))

(event `self.DamageArea.OnComponentBeginOverlap`
  (params (OverlappedComponent :type "PrimitiveComponent Object Reference") (OtherActor :type "Actor Object Reference") (OtherComp :type "PrimitiveComponent Object Reference") (OtherBodyIndex :type Integer) (bFromSweep :type Boolean) (SweepResult :type "HitResult Structure (by ref)"))
  (if (`self.ActorHasTag` OtherActor "Character")
    _))

(fn `UserConstructionScript`)