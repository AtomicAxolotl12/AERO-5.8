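; BP_CorruptionEnemy is an enemy that damages actors tagged "Character" on contact.
; Overlaps with its Sphere2 and Box components each apply a fixed, heavy hit of damage to the tagged actor.
; On BeginPlay it offsets its capsule once by the DeltaTransform value, with sweep enabled; it has no active Tick or other movement logic in its graphs.
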(event `self.ReceiveBeginPlay`
  (`SceneComponent.K2_AddLocalTransform` (`self.CapsuleComponent`) (`self.Delta Transform`) true false))

(event `self.Sphere2.OnComponentBeginOverlap`
  (params (OverlappedComponent :type "PrimitiveComponent Object Reference") (OtherActor :type "Actor Object Reference") (OtherComp :type "PrimitiveComponent Object Reference") (OtherBodyIndex :type Integer) (bFromSweep :type Boolean) (SweepResult :type "HitResult Structure (by ref)"))
  (if (`self.ActorHasTag` OtherActor "Character")
    (`GameplayStatics.ApplyDamage` OtherActor 100.0)))

(event `self.Box.OnComponentBeginOverlap`
  (params (OverlappedComponent :type "PrimitiveComponent Object Reference") (OtherActor :type "Actor Object Reference") (OtherComp :type "PrimitiveComponent Object Reference") (OtherBodyIndex :type Integer) (bFromSweep :type Boolean) (SweepResult :type "HitResult Structure (by ref)"))
  (if (`self.ActorHasTag` OtherActor "Character")
    (`GameplayStatics.ApplyDamage` OtherActor 100.0)))

(fn `UserConstructionScript`)