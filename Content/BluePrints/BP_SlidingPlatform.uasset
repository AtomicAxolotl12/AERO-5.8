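; Sliding platform actor whose mesh travels back and forth between Start and End components.
; A Timeline lerps the mesh's world location, and on finish waits briefly, flips IsGoingForward and calls Forward or Backward to ping-pong.
; StartForward and StartBackward restart it from either end; nothing in this graph triggers the first move.
; Separately, Tick raises the mesh at Speed until its relative Z exceeds Distance.
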(event `self.ReceiveTick`
  (params (DeltaSeconds :type "Float (single-precision)"))
  (bind (_relativelocation_x _relativelocation_y _relativelocation_z) (`KismetMathLibrary.BreakVector` (`SceneComponent.RelativeLocation` (`self.PlatformMesh`))))
  (if (not (> _relativelocation_z (`self.Distance`)))
    (`SceneComponent.K2_AddRelativeLocation` (`self.PlatformMesh`) (`KismetMathLibrary.MakeVector` 0.0 0.0 (* DeltaSeconds (`self.Speed`))) false false)))

(event `Forward`
  (bind (_direction _newtrack_0) (`Timeline|Timeline` :!label _label)
    (:`Update`
      (`SceneComponent.K2_SetWorldLocation` (`self.PlatformMesh`) (`KismetMathLibrary.VLerp` (`SceneComponent.K2_GetComponentLocation` (`self.start`)) (`SceneComponent.K2_GetComponentLocation` (`self.end`)) _newtrack_0) false false))
    (:`Finished`
      (`KismetSystemLibrary.Delay` 0.6)
      (if (`self.Is Going Forward`)
        (set `self.Is Going Forward` false)
        (`self.Backward`)
        (else
          (set `self.Is Going Forward` true)
          (`self.Forward`))))))

(event `StartForward`
  (goto _label :!via `PlayFromStart`))

(event `Backward`
  (goto _label :!via `Reverse`))

(event `StartBackward`
  (goto _label :!via `ReverseFromEnd`))

(fn `UserConstructionScript`
  (`parent.UserConstructionScript`))